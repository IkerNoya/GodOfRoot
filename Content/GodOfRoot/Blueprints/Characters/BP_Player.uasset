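; Player character Blueprint that handles the death and hit reactions of the player.
; Death disables input, ragdolls the mesh, plays death music through the game mode's MusicManager, then opens the menu level after a delay.
; Taking damage plays a hit montage with camera shake and a hurt sound, blocking attacks in CombatComponent until the montage completes, blends out or is interrupted.
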(event EventDie
  (Input|DisableInput (Game|GetPlayerController 0))
  (Physics|SetSimulatePhysics (Variables|Character|GetMesh) true)
  (Collision|SetCollisionEnabled (Variables|Character|GetMesh) "QueryAndPhysics")
  (bind _asbp_main_game_mode (Utilities|Casting|CastToBP_MainGameMode (Game|GetGameMode)))
  (Default|PlayDeath (Variables|/Game/GodOfRoot/Blueprints/Core/BP_MainGameMode.BP_MainGameMode_C|GetMusicManager _asbp_main_game_mode))
  (Utilities|FlowControl|Delay 5.0)
  (Game|OpenLevel(byObjectReference) "/Game/GodOfRoot/Levels/L_Menu.L_Menu"))

(event EventOnDamageReceived
  (params (DamageInstigator :type Actor%20Object%20Reference) (DamageCause :type Object%20Object%20Reference))
  (Animation|Montage|PlayMontage (Variables|Character|GetMesh) "/Game/GodOfRoot/Blueprints/Animations/Montages/AM_Hit1.AM_Hit1" 2.0 0.0 "Default"
    (:then
      (Variables|/Script/GodOfRoot.CombatComponent|SetbCanAttack (Variables|Default|GetCombatComponent) false)
      (Camera|PlayWorldCameraShake "/Game/GodOfRoot/Blueprints/screenShakes/CS_GetHit.CS_GetHit_C" (Transformation|GetWorldLocation (Variables|Default|GetFollowCamera)) 0.0 5e+02)
      (Audio|PlaySound2D "/Game/GodOfRoot/Audio/CUE_PlayerHurt.CUE_PlayerHurt" 1.0 1.0 0.0 0 0))
    (:OnCompleted
      (Variables|/Script/GodOfRoot.CombatComponent|SetbCanAttack (Variables|Default|GetCombatComponent) true :!label _label))
    (:OnBlendOut
      (goto _label))
    (:OnInterrupted
      (goto _label))))

(fn ConstructionScript)
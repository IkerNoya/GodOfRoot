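; Main game mode that handles the victory condition: the level is won when the BP_Sauce actor dies.
; On BeginPlay it binds to the death delegate on the first BP_Sauce's GORHealthComponentBase and caches the level's BP_MusicManager.
; When that death fires, it plays the victory music, waits a few seconds, then opens the L_Menu level.
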(event Custom|OnDeathDelegate_Event_0
  (Default|PlayVictory (Variables|Default|GetMusicManager))
  (Utilities|FlowControl|Delay 8.0)
  (Game|OpenLevel(byObjectReference) "/Game/GodOfRoot/Levels/L_Menu.L_Menu"))

(event EventBeginPlay
  (bind _outactors (Actor|GetAllActorsOfClass "/Game/GodOfRoot/Blueprints/Characters/BP_Sauce.BP_Sauce_C"))
  (EventDispatchers|AssignOnDeathDelegate (Actor|GetComponentbyClass (Utilities|Array|Get(acopy) _outactors) "/Script/GodOfRoot.GORHealthComponentBase") (delegate Custom|OnDeathDelegate_Event_0))
  (bind _returnvalue (Actor|GetActorOfClass "/Game/GodOfRoot/Audio/BP_MusicManager.BP_MusicManager_C"))
  (Variables|Default|SetMusicManager _returnvalue))

(fn ConstructionScript)